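; BP_TimerBlock is a block that periodically vanishes and reappears, releasing the player's hook if one has struck it.
; On BeginPlay, if TimerSeconds is below MaxSeconds, a looping timer starts with a once-randomized interval and toggles visibility and Cube collision between none and query-only.
; Cube hits by BP_Hook are stored in HitActor; hiding with a valid HitActor calls EndHook on the player's RogueCharacter.
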(event OnComponentHit(Cube)
  (params (HitComponent :type Primitive%20Component%20Object%20Reference) (OtherActor :type Actor%20Object%20Reference) (OtherComp :type Primitive%20Component%20Object%20Reference) (NormalImpulse :type Vector :default "0, 0, 0") (Hit :type Hit%20Result%20Structure%20%28by%20ref%29))
  (bind _asbp_hook (Utilities|Casting|CastToBP_Hook OtherActor))
  (Variables|Default|SetHitActor _asbp_hook))

(event Custom|커스텀이벤트
  (bind _cube (Variables|Default|GetCube))
  (bind _output_get (Variables|Default|SetActor%20Hidden%20in%20Game (not (Variables|Rendering|GetbHidden))))
  (Rendering|SetActorHiddenInGame _output_get)
  (if (Variables|Default|GetActor%20Hidden%20in%20Game)
    (Collision|SetCollisionEnabled _cube "NoCollision")
    (Variables|Default|GetHitActor
      (:then
        (bind _asrogue_character (Utilities|Casting|CastToRogueCharacter (Game|Player|GetPlayerPawn 0)))
        (Class|RogueCharacter|EndHook _asrogue_character))
      (:else))
    (else
      (Collision|SetCollisionEnabled _cube "QueryOnly")))
  (Variables|Default|SetHitActor 0))

(event EventBeginPlay
  (if (< (Variables|Default|GetTimerSeconds) (Variables|Default|GetMaxSeconds))
    (Utilities|Time|SetTimerbyEvent (delegate Custom|커스텀이벤트) (Math|Conversions|ToFloat(Integer) (+ (Variables|Default|GetTimerSeconds) (Math|Random|RandomIntegerinRange 0 3))) true)))

(event Collision|EventActorBeginOverlap
  (params (OtherActor :type Actor%20Object%20Reference)))

(event EventTick
  (params (DeltaSeconds :type Float%20%28single-precision%29)))

(fn ConstructionScript)