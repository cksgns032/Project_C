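; BP_Hook is a grappling hook actor that pulls the player character toward the point where it lands.
; BeginPlay attaches the cable's end to BP_MainChar; a capsule hit on a visible actor shows the cable, notifies the character and starts a timer that later calls EndHook.
; After a hit, Tick applies constant force toward the hook and sets cable length from the character's distance, capped at a maximum.
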(event OnComponentHit(CapsuleCollider)
  (params (HitComponent :type Primitive%20Component%20Object%20Reference) (OtherActor :type Actor%20Object%20Reference) (OtherComp :type Primitive%20Component%20Object%20Reference) (NormalImpulse :type Vector :default "0, 0, 0") (Hit :type Hit%20Result%20Structure%20%28by%20ref%29))
  (bind __main_char (Variables|Default|Get%20Main%20Char))
  (if (not (Variables|/Script/Engine.Actor|GetbHidden OtherActor))
    (Variables|Default|SetHit%20Location (.location Hit))
    (Variables|Default|SetApplyForce true)
    (bind _cablecom (Variables|Default|GetCableCom)
      (:then
        (Rendering|SetVisibility _cablecom true false)
        (Utilities|FlowControl|Sequence
          (:then_0
            (Class|RogueCharacter|EndAni __main_char)
            (Development|PrintString "Hit"))
          (:then_1
            (Variables|/Script/CharacterMove.RogueCharacter|SetIsGetTarget __main_char true))
          (:then_2
            (bind _returnvalue (Utilities|Time|SetTimerbyEvent (delegate Custom|Evnet%20Destroy) 3.0))
            (Variables|Default|SetTimerHandle _returnvalue))))
      (:else))))

(event Custom|Evnet%20Destroy
  (Class|RogueCharacter|EndHook (Variables|Default|Get%20Main%20Char))
  (Development|PrintString "Clear"))

(event EventBeginPlay
  (Utilities|Time|ClearandInvalidateTimerbyHandle (Variables|Default|GetTimerHandle))
  (bind _asbp_main_char (Utilities|Casting|CastToBP_MainChar (Game|Player|GetPlayerPawn 0)))
  (Variables|Default|Set%20Main%20Char _asbp_main_char)
  (Class|CableComponent|SetAttachEndto (Variables|Default|GetCableCom) (Variables|Default|Get%20Main%20Char) "Sphere" "None"))

(event Collision|EventActorBeginOverlap
  (params (OtherActor :type Actor%20Object%20Reference)))

(event EventTick
  (params (DeltaSeconds :type Float%20%28single-precision%29))
  (if (Variables|Default|GetApplyForce)
    (Physics|AddForce (Variables|/Script/Engine.Character|GetCharacterMovement (Variables|Default|Get%20Main%20Char)) (* (Math|Vector|Normalize (Math|Vector|GetUnitDirection(Vector) (Transformation|GetActorLocation (Variables|Default|Get%20Main%20Char)) (Transformation|GetActorLocation))) 2e+05))
    (CallFunction|SetCableLength)))

(fn ConstructionScript)

(fn SetCableLength
  (bind __main_char (Variables|Default|Get%20Main%20Char))
  (bind _meshcom (Variables|Default|GetMeshCom))
  (bind _cablecom (Variables|Default|GetCableCom))
  (bind _returnvalue (Transformation|GetActorLocation __main_char))
  (bind _returnvalue_2 (Transformation|GetWorldLocation _meshcom))
  (bind _returnvalue_3 (Math|Vector|Distance(Vector) _returnvalue _returnvalue_2))
  (if (>= _returnvalue_3 1e+02)
    (Variables|/Script/CableComponent.CableComponent|SetCableLength _cablecom 1e+02)
    (else
      (Variables|/Script/CableComponent.CableComponent|SetCableLength _cablecom _returnvalue_3))))

(fn CheckDistance
  (return (>= (Math|Vector|Distance(Vector) (Transformation|GetActorLocation (Variables|Default|Get%20Main%20Char)) (Transformation|GetWorldLocation (Variables|Default|GetMeshCom))) 1e+03)))