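; BP_Panel is an actor that continuously seesaws on its pitch axis between about -14 and +14 degrees.
; Each Tick reads the current pitch and steps it by a fixed amount, flipping the IsUp flag at either limit to reverse direction.
; The step ignores delta time, so the tilt speed depends on frame rate.
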(event EventBeginPlay
  (Variables|Default|SetIsUp false))

(event Collision|EventActorBeginOverlap
  (params (OtherActor :type Actor%20Object%20Reference)))

(event EventTick
  (params (DeltaSeconds :type Float%20%28single-precision%29))
  (Variables|Default|SetReturn%20Value%20Y%20%28Pitch%29 (.pitch (Transformation|GetActorRotation)))
  (if (Variables|Default|GetIsUp)
    (if (>= (Variables|Default|GetReturn%20Value%20Y%20%28Pitch%29) 14.0)
      (Variables|Default|SetIsUp false)
      (else
        (Transformation|SetActorRotation (Math|Rotator|MakeRotator 0.0 (+ (Variables|Default|GetReturn%20Value%20Y%20%28Pitch%29) 0.3) 0.0))))
    (elif (<= (Variables|Default|GetReturn%20Value%20Y%20%28Pitch%29) -14.0)
      (Variables|Default|SetIsUp true)
      (else
        (Transformation|SetActorRotation (Math|Rotator|MakeRotator 0.0 (- (Variables|Default|GetReturn%20Value%20Y%20%28Pitch%29) 0.3) 0.0))))))

(fn ConstructionScript)