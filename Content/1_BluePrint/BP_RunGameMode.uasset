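; Game mode for a run that spawns a limited number of BP_RoguePreview enemies around the player.
; BeginPlay starts a looping timer that calls SpawnEnemy every few seconds and sets GameTime, which is not read here.
; SpawnEnemy places each enemy at a random X/Y offset from the player at the same height and increments EnemyCnt.
; Once the count reaches its cap, it calls ClearTimerByFunctionName instead of spawning.
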(event Custom|Spawn%20Enemy
  (bind _returnvalue (Game|GetPlayerCharacter 0))
  (bind _returnvalue_2 (Transformation|GetActorLocation _returnvalue))
  (bind (_x _y _z) (Math|Vector|BreakVector _returnvalue_2))
  (if (< (Variables|Default|GetEnemyCnt) 10)
    (Game|SpawnActorfromClass "/Game/1_BluePrint/Character/BP_RoguePreview.BP_RoguePreview_C" (Math|Transform|MakeTransform (Math|Vector|MakeVector (Math|Random|RandomFloatinRange (- _x 3e+02) (+ _x 3e+02)) (Math|Random|RandomFloatinRange (- _y 3e+02) (+ _y 3e+02)) _z) "0, 0, 0" "1.000000,1.000000,1.000000") "Undefined" "MultiplyWithRoot" 0 0)
    (Math|Integer|IncrementInt (Variables|Default|GetEnemyCnt))
    (else
      (Utilities|Time|ClearTimerbyFunctionName 0 "Spawn Enemy"))))

(event EventBeginPlay
  (Utilities|Time|SetTimerbyEvent (delegate Custom|Spawn%20Enemy) 3.0 true)
  (Variables|Default|SetGameTime 6e+02))

(event EventTick
  (params (DeltaSeconds :type Float%20%28single-precision%29)))

(fn ConstructionScript)