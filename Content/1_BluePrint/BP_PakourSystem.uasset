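; Parkour component that vaults or front-flips its owning character over obstacles.
; TriggerPakour detects a wall ahead with stacked sphere traces, then scans its top, far edge and landing point.
; If grounded, TryPakour picks one-hand vault, two-hand vault or flip by wall height.
; TryVault plays the montage in flying mode without capsule collision until blend-out, setting motion warp targets for all but the one-hand vault.
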(event Custom|Try%20Vault
  (params (NewParam :type E_ValueType%20Enum :default "NewEnumerator0"))
  (Variables|Default|SetCan%20Pakour false)
  (Collision|SetCollisionEnabled (Variables|Default|GetPlayerCollider) "NoCollision")
  (Pawn|Components|CharacterMovement|SetMovementMode (Variables|Default|GetCharacterMovement) "MOVE_Flying" 0)
  (switch Utilities|FlowControl|Switch|SwitchonE_ValueType NewParam
    (:NewEnumerator0
      (Variables|Default|SetMontage "/Game/3_Animation/OneHandVault_Montage.OneHandVault_Montage"))
    (:NewEnumerator1
      (Variables|Default|SetMontage "/Game/3_Animation/TwoHandVault_Montage.TwoHandVault_Montage")
      (Class|MotionWarpingComponent|AddorUpdateWarpTargetfromLocationandRotation (Variables|Default|GetMotion) "Start" (CallFunction|DownWard (CallFunction|ForWard (.Location (Collision|BreakHitResult (Variables|Default|GetFirstTopHit))) (Variables|Default|GetWallRotation) 1e+02) 4e+01) (Variables|Default|GetWallRotation))
      (Class|MotionWarpingComponent|AddorUpdateWarpTargetfromLocationandRotation (Variables|Default|GetMotion) "End" (.Location (Collision|BreakHitResult (Variables|Default|GetLandingHit))) (Variables|Default|GetWallRotation)))
    (:NewEnumerator2
      (Variables|Default|SetMontage "/Game/3_Animation/FrontFlip_Montage.FrontFlip_Montage")
      (Class|MotionWarpingComponent|AddorUpdateWarpTargetfromLocationandRotation (Variables|Default|GetMotion) "Start" (CallFunction|BackWard (.Location (Collision|BreakHitResult (Variables|Default|GetFirstTopHit))) (Variables|Default|GetWallRotation) 1e+02) (Variables|Default|GetWallRotation))
      (Class|MotionWarpingComponent|AddorUpdateWarpTargetfromLocationandRotation (Variables|Default|GetMotion) "End" (CallFunction|RightWard (.Location (Collision|BreakHitResult (Variables|Default|GetLandingHit))) (Variables|Default|GetWallRotation) 5.0) (Variables|Default|GetWallRotation))))
  (Animation|Montage|PlayMontage (Variables|Default|GetPlayerMesh) (Variables|Default|GetMontage)
    (:OnCompleted
      (Variables|Default|SetCan%20Pakour true))
    (:OnBlendOut
      (Collision|SetCollisionEnabled (Variables|Default|GetPlayerCollider) "QueryAndPhysics")
      (Pawn|Components|CharacterMovement|SetMovementMode (Variables|Default|GetCharacterMovement) "MOVE_Walking" 0))))

(event EventTick
  (params (DeltaSeconds :type Float%20%28single-precision%29))
  (bind _playermesh (Variables|Default|GetPlayerMesh))
  (bind _returnvalue (Transformation|GetWorldLocation _playermesh))
  (bind _returnvalue_2 (Collision|SphereTraceByChannel _returnvalue _returnvalue (Variables|/Script/Engine.CapsuleComponent|GetCapsuleRadius (Variables|Default|GetPlayerCollider)) "TraceTypeQuery1" false 0 "ForOneFrame"))
  (Variables|Default|SetIs%20On%20Land _returnvalue_2))

(fn TriggerPakour
  (bind (_return _hitlocation _reversenormal) (CallFunction|DetectWall))
  (if _return
    (CallFunction|ScanWall _hitlocation _reversenormal)
    (CallFunction|TryPakour)))

(fn DetectWall
  (bind _returnvalue (Components|GetOwner))
  (bind _index (Utilities|FlowControl|ForLoopwithBreak 0 7 :!label _label)
    (:LoopBody
      (bind (_outhit _returnvalue_2) (Collision|SphereTraceByChannel (CallFunction|BackWard (CallFunction|UpWard (CallFunction|DownWard (Transformation|GetActorLocation _returnvalue) 6e+01) (* _index 20)) (Transformation|GetActorRotation _returnvalue) 3e+01) (+ (CallFunction|UpWard (CallFunction|DownWard (Transformation|GetActorLocation _returnvalue) 6e+01) (* _index 20)) (* (Transformation|GetActorForwardVector _returnvalue) 2e+02)) 1e+01 "TraceTypeQuery1" false 0 "ForOneFrame"))
      (if _returnvalue_2
        (Utilities|FlowControl|Sequence
          (:then_0
            (goto _label Break))
          (:then_1
            (return (.bBlockingHit (Collision|BreakHitResult _outhit)) (.Location (Collision|BreakHitResult _outhit)) (CallFunction|ReverseNormal (.Normal (Collision|BreakHitResult _outhit))))))))))

(fn ScanWall
  (params (Vector :type Vector) (Rotator :type Rotator))
  (bind _index (Utilities|FlowControl|ForLoopwithBreak 0 29 :!label _label)
    (:LoopBody
      (bind (_outhit _returnvalue) (Collision|LineTraceByChannel (CallFunction|BackWard (CallFunction|DownWard (CallFunction|UpWard Vector 3e+02) (* _index 10)) Rotator 2e+01) (CallFunction|ForWard (CallFunction|DownWard (CallFunction|UpWard Vector 3e+02) (* _index 10)) Rotator 8e+01) "TraceTypeQuery1" false 0 "ForOneFrame"))
      (if _returnvalue
        (Variables|Default|SetScanHit _outhit)
        (goto _label Break)))
    (:Completed
      (Variables|Default|SetWallRotation (CallFunction|ReverseNormal (.Normal (Collision|BreakHitResult (Variables|Default|GetScanHit)))))
      (bind _index_2 (Utilities|FlowControl|ForLoopwithBreak 0 9 :!label _label_2)
        (:LoopBody
          (bind (_outhit_2 _returnvalue_2) (Collision|SphereTraceByChannel (CallFunction|UpWard (CallFunction|ForWard (.Location (Collision|BreakHitResult (Variables|Default|GetScanHit))) (Variables|Default|GetWallRotation) (* _index_2 20)) 1e+01) (CallFunction|DownWard (CallFunction|UpWard (CallFunction|ForWard (.Location (Collision|BreakHitResult (Variables|Default|GetScanHit))) (Variables|Default|GetWallRotation) (* _index_2 20)) 1e+01) 1e+01) 5.0 "TraceTypeQuery1" false 0 "ForOneFrame"))
          (if (== _index_2 0)
            (if _returnvalue_2
              (Variables|Default|SetFirstTopHit _outhit_2))
            (elif _returnvalue_2
              (Variables|Default|SetLastTopHit _outhit_2)
              (else
                (Utilities|FlowControl|Sequence
                  (:then_0
                    (goto _label_2 Break))
                  (:then_1
                    (bind (_outhit_3 _returnvalue_3) (Collision|SphereTraceByChannel (CallFunction|ForWard (.ImpactPoint (Collision|BreakHitResult (Variables|Default|GetLastTopHit))) (Variables|Default|GetWallRotation) 2e+01) (.ImpactPoint (Collision|BreakHitResult (Variables|Default|GetLastTopHit))) 1e+01 "TraceTypeQuery1" false 0 "None"))
                    (if _returnvalue_3
                      (bind _output_get (Variables|Default|SetEnd%20Wall%20Hit _outhit_3))
                      (bind (_outhit_4 _returnvalue_4) (Collision|SphereTraceByChannel (CallFunction|ForWard (.ImpactPoint (Collision|BreakHitResult _output_get)) (Variables|Default|GetWallRotation) 6e+01) (CallFunction|DownWard (CallFunction|ForWard (.ImpactPoint (Collision|BreakHitResult _output_get)) (Variables|Default|GetWallRotation) 6e+01) 1.8e+02) 1e+01 "TraceTypeQuery1" false 0 "None"))
                      (if _returnvalue_4
                        (Variables|Default|SetLandingHit _outhit_4)))))))))))))

(fn MeasureWall
  (if (and (.bBlockingHit (Collision|BreakHitResult (Variables|Default|GetScanHit))) (.bBlockingHit (Collision|BreakHitResult (Variables|Default|GetFirstTopHit))))
    (Variables|Default|SetWallHeight (- (.Z (Math|Vector|BreakVector (.ImpactPoint (Collision|BreakHitResult (Variables|Default|GetFirstTopHit))))) (.Z (Math|Vector|BreakVector (Transformation|GetWorldLocation (Variables|Default|GetPlayerMesh))))))
    (else
      (Variables|Default|SetWallHeight 0.0))))

(fn Init
  (bind _return (Class|BPIPlayer|GetMesh(Message) (Components|GetOwner)))
  (Variables|Default|SetPlayerMesh _return)
  (bind _newparam (Class|BPIPlayer|GetCollider(Message) (Components|GetOwner)))
  (Variables|Default|SetPlayerCollider _newparam)
  (bind _newparam_2 (Class|BPIPlayer|GetCharacterMovement(Message) (Components|GetOwner)))
  (Variables|Default|SetCharacterMovement _newparam_2)
  (bind _newparam_3 (Class|BPIPlayer|GetMotion(Message) (Components|GetOwner)))
  (Variables|Default|SetMotion _newparam_3))

(fn TryPakour
  (bind _wallheight (Variables|Default|GetWallHeight))
  (if (.bBlockingHit (Collision|BreakHitResult (Variables|Default|GetFirstTopHit)))
    (if (Variables|Default|GetIs%20On%20Land)
      (CallFunction|MeasureWall)
      (if (<= (Variables|Default|GetWallHeight) 3e+02)
        (if (>= (Variables|Default|GetWallHeight) 1.3e+02)
          (CallFunction|TryVault "NewEnumerator2")
          (elif (> _wallheight 9e+01)
            (CallFunction|TryVault "NewEnumerator1")
            (else
              (CallFunction|TryVault "NewEnumerator0"))))
        (Development|PrintString (Utilities|String|ToString(Float) _wallheight))))))