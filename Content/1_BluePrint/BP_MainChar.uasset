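; Main character Blueprint whose only live logic draws a debug capsule every Tick, matching its collision capsule.
; The remaining logic sits in disconnected fragments that never run.
; These hold a cable grapple that extends the cable and pulls the character by force, toggles between collisionless Flying and query-only Walking or Falling, and a Motion Warping "End" target placed ahead of the character.
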(event EventBeginPlay)

(event Collision|EventActorBeginOverlap
  (params (OtherActor :type Actor%20Object%20Reference)))

(event EventTick
  (params (DeltaSeconds :type Float%20%28single-precision%29))
  (bind _capsulecomponent (Variables|Default|GetCapsuleComponent))
  (Rendering|Debug|DrawDebugCapsule (Transformation|GetActorLocation) (Variables|/Script/Engine.CapsuleComponent|GetCapsuleHalfHeight _capsulecomponent) (Variables|/Script/Engine.CapsuleComponent|GetCapsuleRadius _capsulecomponent) (Transformation|GetActorRotation) "(R=1.000000,G=1.000000,B=1.000000,A=1.000000)" 0.0 0.0))

(fn ConstructionScript)