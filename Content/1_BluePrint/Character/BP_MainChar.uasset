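; Main player character Blueprint with a rope hook action and a trace-based climb-up move.
; IA_ROPE spawns a BP_Hook along the view direction when grounded and allowed, and calls EndHook on release.
; C sphere-traces ahead at stacked heights, capsule-traces for a stand point, then plays a motion-warped climb montage, switching between Flying and Falling.
; Tick draws the debug capsule; item hold-to-charge interaction logic is present but unconnected.
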(event Input|EnhancedActionEvents|EnhancedInputActionIA_ROPE
  (params (ActionValue :type Boolean) (ElapsedSeconds :type Float%20%28double-precision%29) (TriggeredSeconds :type Float%20%28double-precision%29) (InputAction :type Input%20Action%20Object%20Reference :default "/Game/4_Input/IA_ROPE.IA_ROPE"))
  (bind _returnvalue (Pawn|GetController))
  (bind _rotation (Pawn|GetPlayerViewPoint _returnvalue))
  ;[1 1 1] 로프 액션
  (:Started
    (if (and (not (Variables|Default|GetIsAirbon)) (Variables|Default|GetCanRope))
      (Variables|Default|SetCanRope false)
      (bind _returnvalue_2 (Game|SpawnActorfromClass "/Game/1_BluePrint/Actor/BP_Hook.BP_Hook_C" (Math|Transform|MakeTransform (+ (Transformation|GetActorLocation) (Math|Vector|Normalize (Math|Vector|GetForwardVector _rotation))) _rotation "1.000000,1.000000,1.000000") "Undefined" "MultiplyWithRoot" 0 (* (Math|Rotator|GetRotationXVector _rotation) 0.5) 0))
      (Variables|Default|SetHook _returnvalue_2)))
  (:Completed
    (Class|RogueCharacter|EndHook)))

(event EventBeginPlay)

(event Collision|EventActorBeginOverlap
  (params (OtherActor :type Actor%20Object%20Reference)))

(event EventTick
  (params (DeltaSeconds :type Float%20%28single-precision%29))
  (bind _capsulecomponent (Variables|Default|GetCapsuleComponent))
  ;[1 1 1] 캐릭터 캡슐 콜라이더
  (Rendering|Debug|DrawDebugCapsule (Transformation|GetActorLocation) (Variables|/Script/Engine.CapsuleComponent|GetCapsuleHalfHeight _capsulecomponent) (Variables|/Script/Engine.CapsuleComponent|GetCapsuleRadius _capsulecomponent) (Transformation|GetActorRotation) "(R=1.000000,G=1.000000,B=1.000000,A=1.000000)" 0.0 0.0))

(event Input|KeyboardEvents|C
  (params (Key :type Key%20Structure :default "None"))
  (bind _mesh (Variables|Character|GetMesh))
  (bind _capsulecomponent (Variables|Default|GetCapsuleComponent))
  (bind _charactermovement (Variables|Character|GetCharacterMovement))
  (bind _returnvalue (Transformation|GetWorldLocation _mesh))
  (bind (_x _y _z) (Math|Vector|BreakVector _returnvalue))
  (:Pressed
    (Class|RogueCharacter|EndAni)
    ;[1 1 1] Front Search
    (Variables|Default|SetFirst%20Hit%20 "")
    (bind _index (Utilities|FlowControl|ForLoopwithBreak 1 4 :!label _label)
      (:LoopBody
        (bind (_outhit _returnvalue_2) (Collision|SphereTraceByChannel (Math|Vector|MakeVector _x _y (+ (* _index 30) (+ _z 1e+02))) (+ (Math|Vector|MakeVector _x _y (+ (* _index 30) (+ _z 1e+02))) (* (Math|Vector|Normalize (Math|Vector|GetForwardVector (Transformation|GetActorRotation))) 1e+02)) 6.0 "TraceTypeQuery1" false 0 "ForDuration"))
        (if _returnvalue_2
          (Variables|Default|SetFirst%20Hit%20 _outhit)
          (else
            (goto _label Break))))
      (:Completed
        ;[1 1 1] Stand Point Search
        (if (.bBlockingHit (Collision|BreakHitResult (Variables|Default|GetFirst%20Hit%20)))
          (Variables|Default|SetStand%20Hit "")
          (bind _index_2 (Utilities|FlowControl|ForLoopwithBreak 0 7 :!label _label_2)
            (:LoopBody
              (bind (_outhit_2 _returnvalue_3) (Collision|CapsuleTraceByChannel (.ImpactPoint (Collision|BreakHitResult (Variables|Default|GetFirst%20Hit%20))) (+ (.ImpactPoint (Collision|BreakHitResult (Variables|Default|GetFirst%20Hit%20))) (* (Math|Vector|Normalize (Math|Vector|GetForwardVector (Transformation|GetActorRotation))) (* _index_2 20))) 6.0 12.0 "TraceTypeQuery1" false 0 "ForDuration"))
              (if _returnvalue_3
                (Variables|Default|SetStand%20Hit _outhit_2)
                (goto _label_2 Break)
                (else
                  (Variables|Default|SetStand%20Hit _outhit_2))))
            (:Completed
              ;[1 1 1] Play Climb Montage
              (if (.bBlockingHit (Collision|BreakHitResult (Variables|Default|GetStand%20Hit)))
                (Class|MotionWarpingComponent|AddorUpdateWarpTargetfromLocationandRotation (Variables|Default|GetMotionWarping) "Stand_Location" (.Location (Collision|BreakHitResult (Variables|Default|GetStand%20Hit))) (Transformation|GetActorRotation))
                (Animation|Montage|PlayMontage (Variables|Character|GetMesh) "/Game/3_Animation/AM_ClimbUp.AM_ClimbUp"
                  (:then
                    (Collision|SetCollisionEnabled _capsulecomponent "QueryAndPhysics")
                    (Pawn|Components|CharacterMovement|SetMovementMode _charactermovement "MOVE_Flying" 0))
                  (:OnBlendOut
                    (Collision|SetCollisionEnabled _capsulecomponent "QueryAndPhysics")
                    (Pawn|Components|CharacterMovement|SetMovementMode _charactermovement "MOVE_Falling" 0)))))))))))

(event Input|KeyboardEvents|E
  (params (Key :type Key%20Structure :default "None")))

(fn ConstructionScript)