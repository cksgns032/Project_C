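; BP_Helper is a set of vector math helper functions for offsetting positions and turning a direction into a rotation.
; UpWard and DownWard shift a vector along world Z.
; ForWard, BackWard, LeftWard and RightWard shift it along the forward or right axis of a given rotation.
; ReverseNormal builds a rotator from a vector's X axis and applies a 180-degree delta on one component.
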(fn UpWard
  (params (Vector%20 :type Vector) (Add :type Float%20%28double-precision%29))
  (return (+ Vector%20 (Math|Vector|MakeVector 0.0 0.0 Add))))

(fn DownWard
  (params (Vector :type Vector) (Minus :type Float%20%28double-precision%29))
  (return (- Vector (Math|Vector|MakeVector 0.0 0.0 Minus))))

(fn ForWard
  (params (Vector :type Vector) (Rotation :type Rotator) (Add :type Float%20%28double-precision%29))
  (return (+ Vector (* (Math|Vector|GetForwardVector Rotation) Add))))

(fn BackWard
  (params (Vector :type Vector) (Rotator :type Rotator) (Minus :type Float%20%28double-precision%29))
  (return (- Vector (* (Math|Vector|GetForwardVector Rotator) Minus))))

(fn LeftWard
  (params (Vector :type Vector) (Rotator :type Rotator) (Value :type Float%20%28double-precision%29))
  (return (- Vector (* (Math|Vector|GetRightVector Rotator) Value))))

(fn RightWard
  (params (Vectro :type Vector) (Rotator :type Rotator) (Value :type Float%20%28double-precision%29))
  (return (+ Vectro (* (Math|Vector|GetRightVector Rotator) Value))))

(fn ReverseNormal
  (params (Vector :type Vector))
  (return (Math|Rotator|Delta(Rotator) (Math|Rotator|MakeRotfromX Vector) "0.000000,180.000000,0.000000")))